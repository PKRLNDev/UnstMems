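; BP_Interactables_Frame is a frame actor with an animated spotlight.
; On BeginPlay it calls the parent event, then plays the LightT timeline, whose float track lerps the SpotLight's relative height while X and Y stay fixed.
; The construction script only calls its parent, and the overlap and tick events are disabled stubs.
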(event `self.ReceiveBeginPlay`
  (`parent.ReceiveBeginPlay`)
  (bind (_direction _float) (`Timeline|Light T`)
    (:`Update`
      (`SceneComponent.K2_SetRelativeLocation` (`self.SpotLight`) (`KismetMathLibrary.MakeVector` 268.0 -95.0 (`KismetMathLibrary.Lerp` 120.0 155.0 _float)) false false))))

(fn `UserConstructionScript`
  (`parent.UserConstructionScript`))