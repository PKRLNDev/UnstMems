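; BP_Lever is a lever actor whose arm moves between seven discrete positions.
; Left and Right step the clamped LeverState up or down, and each maps the state to a fixed relative rotation of the Arm through its own duplicated switch.
; Activation snaps the lever to its lowest state.
; The event graph is empty, so these functions only run when called from outside.
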(fn `Activation`
  (set `self.LeverState` -3)
  (`SceneComponent.K2_SetRelativeRotation` (`self.Arm`) (struct :`Pitch` -25.0) false false))

(fn `Left`
  (set `self.LeverState` (`KismetMathLibrary.Clamp` (+ (`self.LeverState`) 1) -3 3))
  (switch `int` (`self.LeverState`)
    (:`-3`
      (`SceneComponent.K2_SetRelativeRotation` (`self.Arm`) (struct :`Pitch` -25.0) false true))
    (:`-2`
      (`SceneComponent.K2_SetRelativeRotation` (`self.Arm`) (struct :`Pitch` -15.0) false true))
    (:`-1`
      (`SceneComponent.K2_SetRelativeRotation` (`self.Arm`) (struct :`Pitch` -5.0) false true))
    (:`0`
      (`SceneComponent.K2_SetRelativeRotation` :`self` (`self.Arm`) :`bTeleport` true))
    (:`1`
      (`SceneComponent.K2_SetRelativeRotation` (`self.Arm`) (struct :`Pitch` 5.0) false true))
    (:`2`
      (`SceneComponent.K2_SetRelativeRotation` (`self.Arm`) (struct :`Pitch` 15.0) false true))
    (:`3`
      (`SceneComponent.K2_SetRelativeRotation` (`self.Arm`) (struct :`Pitch` 25.0) false true))))

(fn `Right`
  (set `self.LeverState` (`KismetMathLibrary.Clamp` (- (`self.LeverState`) 1) -3 3))
  (switch `int` (`self.LeverState`)
    (:`-3`
      (`SceneComponent.K2_SetRelativeRotation` (`self.Arm`) (struct :`Pitch` -25.0) false true))
    (:`-2`
      (`SceneComponent.K2_SetRelativeRotation` (`self.Arm`) (struct :`Pitch` -15.0) false true))
    (:`-1`
      (`SceneComponent.K2_SetRelativeRotation` (`self.Arm`) (struct :`Pitch` -5.0) false true))
    (:`0`
      (`SceneComponent.K2_SetRelativeRotation` :`self` (`self.Arm`) :`bTeleport` true))
    (:`1`
      (`SceneComponent.K2_SetRelativeRotation` (`self.Arm`) (struct :`Pitch` 5.0) false true))
    (:`2`
      (`SceneComponent.K2_SetRelativeRotation` (`self.Arm`) (struct :`Pitch` 15.0) false true))
    (:`3`
      (`SceneComponent.K2_SetRelativeRotation` (`self.Arm`) (struct :`Pitch` 25.0) false true))))

(fn `UserConstructionScript`)