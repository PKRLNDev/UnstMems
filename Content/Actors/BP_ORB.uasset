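; BP_ORB is a glowing orb actor with a dynamic glow material created at BeginPlay.
; EnergyDriver randomizes orbit size, light intensity and material scroll speeds, then starts a timeline that moves the mesh around a Y-Z circle using sine and cosine.
; StateManager routes to up/down handlers that call CallStateChange; dimming only prints a placeholder.
; Glow and height setters exist but are not called here, and ParticlesManager is empty.
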(event `self.ReceiveBeginPlay`
  (`self.CreateAndSetOrbMat`))

(fn `CreateAndSetOrbMat`
  (bind _returnvalue (`KismetMaterialLibrary.CreateDynamicMaterialInstance` "/Game/Mats/M_OrbGlow_Inst.M_OrbGlow_Inst"))
  (bind _output_get (set `self.OrbGlow` _returnvalue))
  (`PrimitiveComponent.SetMaterial` (`self.ORBMESH`) 0 _output_get))

(fn `EnergyDriver`
  (params (State :type Integer))
  (set `self.Diameter` (`KismetMathLibrary.RandomFloatInRange` 200.0 300.0))
  (set `self.Distance` (`KismetMathLibrary.RandomFloatInRange` -20.0 -50.0))
  (set `self.Emition` (`KismetMathLibrary.RandomFloatInRange` 0.0 1000.0))
  (`self.LightControl` (/ (`self.Emition`) 2.0))
  (`self.SpeedControl` (`KismetMathLibrary.RandomFloatInRange` -0.3 0.3) (`KismetMathLibrary.RandomFloatInRange` -0.3 0.3))
  (`TimelineComponent.PlayFromStart` (`self.FloatT`)))

(fn `GlowControl`
  (params (GlowAmount :type "Float (double-precision)"))
  (`MaterialInstanceDynamic.SetScalarParameterValue` (`self.OrbGlow`) (`self.EmitionName`) GlowAmount))

(fn `HeightControl`
  (params (HDistance :type "Float (double-precision)"))
  (`MaterialInstanceDynamic.SetScalarParameterValue` (`self.OrbGlow`) (`self.DistanceName`) HDistance))

(fn `LightControl`
  (params (NewIntensity :type "Float (double-precision)"))
  (`LightComponent.SetIntensity` (`self.PointLight`) (`KismetMathLibrary.RandomFloatInRange` 100.0 500.0)))

(fn `ParticlesManager`)

(fn `SpeedControl`
  (params (SpdX :type "Float (double-precision)") (SpdY :type "Float (double-precision)"))
  (bind _orbglow (`self.OrbGlow`))
  (`MaterialInstanceDynamic.SetScalarParameterValue` _orbglow (`self.SpeedXName`) SpdX)
  (`MaterialInstanceDynamic.SetScalarParameterValue` _orbglow (`self.SpeedYName`) SpdY))

(fn `StateDown`
  (`KismetSystemLibrary.PrintString` "PlayDimmAnim")
  (`self.StateChange` (`self.State`)))

(fn `StateManager`
  (params (UpDown :type Boolean))
  (if UpDown
    (`self.StateUp`)
    (else
      (`self.StateDown`))))

(fn `StateUp`
  (`self.StateChange` (`self.State`)))

(fn `UserConstructionScript`)