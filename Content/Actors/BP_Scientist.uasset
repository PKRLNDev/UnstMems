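; BP_Scientist is an actor that walks along world Y from the Walk axis unless the Crankin timeline is playing.
; Walk does a swept, speed-scaled move, switching off capsule physics and gravity and nudging upward at or below a height threshold.
; Capsule overlaps with BP_Interactables broadcast interaction availability by ID.
; The face-bob timeline and material parameter tweaks are unwired, and Crank, Lever and Interact are empty stubs.
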(event `InputAxis|Walk`
  (params (AxisValue :type "Float (single-precision)"))
  (if (not (`TimelineComponent.IsPlaying` (`self.Crankin`)))
    (`self.Walk` AxisValue)))

(event `self.Capsule.OnComponentBeginOverlap`
  (params (OverlappedComponent :type "PrimitiveComponent Object Reference") (OtherActor :type "Actor Object Reference") (OtherComp :type "PrimitiveComponent Object Reference") (OtherBodyIndex :type Integer) (bFromSweep :type Boolean) (SweepResult :type "HitResult Structure (by ref)"))
  (bind _asbp_interactables (cast `/Game/Actors/BP_Interactables` OtherActor))
  (`self.InteractAvail` (`/Game/Actors/BP_Interactables.ID` _asbp_interactables)))

(event `self.Capsule.OnComponentEndOverlap`
  (params (OverlappedComponent :type "PrimitiveComponent Object Reference") (OtherActor :type "Actor Object Reference") (OtherComp :type "PrimitiveComponent Object Reference") (OtherBodyIndex :type Integer))
  (bind _asbp_interactables (cast `/Game/Actors/BP_Interactables` OtherActor))
  (`self.InteractUnavail` (`/Game/Actors/BP_Interactables.ID` _asbp_interactables)))

(fn `Crank`)

(fn `Interact`)

(fn `Lever`)

(fn `UserConstructionScript`)

(fn `Walk`
  (params (AxisValue :type "Float (double-precision)"))
  (bind (_returnvalue_x _returnvalue_y _returnvalue_z) (`KismetMathLibrary.BreakVector` (`self.K2_GetActorLocation`)))
  (bind _capsule (`self.Capsule`))
  (`self.K2_AddActorWorldOffset` (`KismetMathLibrary.MakeVector` 0.0 (* AxisValue (`GameplayStatics.GetWorldDeltaSeconds`) (`self.WalkSpeed`))) true true)
  (if (<= _returnvalue_z 95.0)
    (`PrimitiveComponent.SetSimulatePhysics` _capsule false)
    (`PrimitiveComponent.SetEnableGravity` _capsule false)
    (`self.K2_AddActorWorldOffset` (0.0 0.0 1.0) true true)))