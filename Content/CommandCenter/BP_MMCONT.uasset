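; BP_MMCONT is the main menu controller, which shows the menu UI and handles muting of its background music.
; On BeginPlay it creates WBP_MainMenu, stores it as MMUI and adds it to the viewport.
; The MuteMusic input toggles BGM by stopping it or playing it from the start, a workaround for volume changes not working, so playback position is not kept.
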(event `self.ReceiveBeginPlay`
  (bind _returnvalue (`|CreateWidget` "/Game/UI/WBP_MainMenu.WBP_MainMenu_C"))
  (bind _output_get (set `self.MMUI` _returnvalue))
  (`UserWidget.AddToViewport` _output_get 0))

(event `InputAction|MuteMusic`
  (params (Key :type "Key Structure"))
  (:`Pressed`
    (`self.MuteUnMuteMusic`)))

(fn `MuteUnMuteMusic`
  (bind _bgm (`self.BGM`))
  ;[1 0 0] #BugFix_6_MainMenuBGM // setting volume to 0~1 wasn't working so i switched to Pause~Unpause
  (if (`AudioComponent.IsPlaying` (`self.BGM`))
    (`AudioComponent.Stop` _bgm)
    (else
      (`AudioComponent.Play` _bgm 0.0))))

(fn `UserConstructionScript`)