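; Player controller for an orb-stabilizing minigame driven by a physical crank and a lever, ending in a manifestation UI.
; Crank spin becomes energy, which lets Interact start the engine once high enough.
; A looping timer compares energy to a timeline-wandered target, growing the orb on mismatch, while lever side versus orb position grows or shrinks it.
; Keeping the orb small builds stabilization, then a timeline counts stability checks before manifesting.
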(event `self.ReceiveBeginPlay`
  (`self.HudSetup`)
  (`self.SetupManifestWidget`)
  (`self.GetActors`)
  (`KismetSystemLibrary.K2_SetTimerDelegate` (`|CreateDelegate` :!event `PsuedoCrankTick`) 0.066667 true))

(event `Key|U`
  (params (Key :type "Key Structure"))
  (bind _manifestui (`self.ManifestUI`))
  ;[1 1 1] Debug
  (:`Pressed`
    (`Widget.SetVisibility` _manifestui "Visible")
    (`UserWidget.PlayAnimation` _manifestui (`/Game/UI/WBP_Manifests.ShowUp` _manifestui) 0.0 1 "Forward" 1.0 false)))

(event `Key|I`
  (params (Key :type "Key Structure"))
  ;[1 1 1] Debug
  (:`Pressed`
    (`Widget.SetVisibility` (`self.ManifestUI`) "Collapsed")))

(event `InputAction|Interact`
  (params (Key :type "Key Structure"))
  (:`Pressed`
    (if (`self.bActive`)
      _
      (elif (> (`self.CurrentEnergy`) (`self.TargetEnergy`))
        (`self.StartEngine`)
        (`self.SetUnstable`)
        (set `self.bActive` true)
        (set `self.ToStability` 0)
        (set `self.ToStabilization` 0)
        (set `self.TargetEnergy` (`KismetMathLibrary.RandomFloatInRange` 50.0 180.0))
        (`/Game/Actors/BP_Crank.Halt` (`self.Crank`) 0.5)
        (`/Engine/EditorBlueprintResources/StandardMacros.DoOnce` false
          (:`Completed`
            (`/Game/Actors/BP_Lever.Activation` (`self.Lever`))))))))

(event `InputAction|Halt`
  (params (Key :type "Key Structure"))
  (:`Pressed`
    (`/Game/Actors/BP_Crank.Torque` (`self.Crank`) -3.0)))

(event `InputAction|Crank`
  (params (Key :type "Key Structure"))
  (:`Pressed`
    (`/Game/Actors/BP_Crank.Torque` (`self.Crank`) 1.0)
    (if (> (`self.CurrentEnergy`) (`self.StartupEnergy`))
      (`/Engine/EditorBlueprintResources/StandardMacros.DoOnce` false :!label _label
        (:`Completed`
          (`KismetSystemLibrary.PrintString` "Press E to Start Engine")))
      (else
        (goto _label :!via `Reset`)))))

(event `PsuedoCrankTick`
  (`self.GetCrankSpeed`)
  (set `self.CurrentEnergy` (* 10 (`self.CrankSpeed`)))
  (if (`self.bActive`)
    ;[1 1 1] EnergyDimDrive
    (`self.DiameterDrive`)
    ;[1 1 1] Stabilization
    (if (`self.CanStabilize`)
      (`self.Stabilize`)
      (else
        ;[1 1 1] LeverDimDrive
        (if (`self.OrbPositiontoLever`)
          (`self.IncreaseDiameter`)
          (`self.Unstabilize` 1.0)
          (else
            (`self.ReduceDiameter`)
            (`self.Unstabilize` 0.5)))))))

(event `InputAction|Left`
  (params (Key :type "Key Structure"))
  ;[1 1 1] LEVER
  (:`Pressed`
    (`/Game/Actors/BP_Lever.Left` (`self.Lever`))))

(event `InputAction|Right`
  (params (Key :type "Key Structure"))
  ;[1 1 1] LEVER
  (:`Pressed`
    (`/Game/Actors/BP_Lever.Right` (`self.Lever`))))

(fn `CanStabilize`
  (returns (ReturnValue :type Boolean))
  (return (and (< (`/Game/Actors/BP_ORB.Diameter` (`self.ORB`)) (`self.DiameterDeadzone`)) (`self.bActive`) (not (`self.bStabilizing`)))))

(fn `CountToStability`
  (bind _orb (`self.ORB`))
  (if (>= (`self.ToStability`) 6)
    (`self.Manifestation`)
    (set `/Game/Actors/BP_ORB.Diameter` 0.0 _orb)
    (`TimelineComponent.Stop` (`/Game/Actors/BP_ORB.FloatT` _orb))
    (set `self.bActive` false)
    (`TimelineComponent.Stop` (`self.Stabilzation`))
    (`KismetSystemLibrary.PrintString` "MoveManifests \nadd inScene Manifests //Ghosts \nGiveInfo=> Interact with Ghost! \n \nShould Make it obvious you should keep the crank going!")
    (else
      (`/Engine/EditorBlueprintResources/StandardMacros.IncrementInt` (`self.ToStability`)))))

(fn `DiameterDrive`
  (bind _orb (`self.ORB`))
  (bind _diameter (`/Game/Actors/BP_ORB.Diameter` _orb))
  (bind _returnvalue (`KismetMathLibrary.Abs` (- (`self.BufferEnergy`) (`self.CurrentEnergy`))))
  (if (> _returnvalue (`self.EnergyDeadzone`))
    (set `/Game/Actors/BP_ORB.Diameter` (`KismetMathLibrary.FClamp` (+ _diameter (* _diameter _returnvalue 0.1)) 0.0 300.0) _orb)))

(fn `GetActors`
  (bind _returnvalue (`GameplayStatics.GetActorOfClass` "/Game/Actors/BP_ORB.BP_ORB_C"))
  (set `self.ORB` _returnvalue)
  (bind _returnvalue_2 (`GameplayStatics.GetActorOfClass` "/Game/Actors/BP_Lever.BP_Lever_C"))
  (set `self.Lever` _returnvalue_2)
  (bind _returnvalue_3 (`GameplayStatics.GetActorOfClass` "/Game/Actors/BP_Crank.BP_Crank_C"))
  (set `self.Crank` _returnvalue_3))

(fn `GetCrankSpeed`
  (bind _returnvalue_x (`KismetMathLibrary.BreakVector` (`PrimitiveComponent.GetPhysicsAngularVelocityInRadians` (`/Game/Actors/BP_Crank.Crank` (`self.Crank`)) "None")))
  (if (> _returnvalue_x 0.0)
    (set `self.CrankSpeed` _returnvalue_x)
    (else
      (set `self.CrankSpeed` 0.0))))

(fn `HudSetup`
  (bind _returnvalue (`|CreateWidget` "/Game/UI/WBP_Accounting.WBP_Accounting_C"))
  (bind _output_get (set `self.HUD` _returnvalue))
  (`UserWidget.AddToViewport` _output_get 0))

(fn `IncreaseDiameter`
  (bind _orb (`self.ORB`))
  (set `/Game/Actors/BP_ORB.Diameter` (`KismetMathLibrary.FClamp` (+ (`/Game/Actors/BP_ORB.Diameter` _orb) (`KismetMathLibrary.Abs` (`KismetMathLibrary.Conv_IntToDouble` (`/Game/Actors/BP_Lever.LeverState` (`self.Lever`))))) 0.0 300.0) _orb))

(fn `IsStable`
  (returns (ReturnValue :type Boolean))
  (return (and (< (`/Game/Actors/BP_ORB.Diameter` (`self.ORB`)) (`self.DiameterDeadzone`)) (`self.bStabilizing`))))

(fn `Manifestation`
  (bind _manifestui (`self.ManifestUI`))
  (`UserWidget.PlayAnimation` _manifestui (`/Game/UI/WBP_Manifests.ShowUp` _manifestui) 0.0 1 "Forward" 1.0 false))

(fn `OrbPositiontoLever`
  (returns (ReturnValue :type Boolean))
  (bind (_relativelocation_x _relativelocation_y) (`KismetMathLibrary.BreakVector` (`SceneComponent.RelativeLocation` (`/Game/Actors/BP_ORB.ORBMESH` (`self.ORB`)))))
  (bind (_relativerotation_roll _relativerotation_pitch) (`KismetMathLibrary.BreakRotator` (`SceneComponent.RelativeRotation` (`/Game/Actors/BP_Lever.Arm` (`self.Lever`)))))
  (bind (_relativelocation_x_2 _relativelocation_y_2) (`KismetMathLibrary.BreakVector` (`SceneComponent.RelativeLocation` (`/Game/Actors/BP_ORB.ORBMESH` (`self.ORB`)))))
  (bind (_relativerotation_roll_2 _relativerotation_pitch_2) (`KismetMathLibrary.BreakRotator` (`SceneComponent.RelativeRotation` (`/Game/Actors/BP_Lever.Arm` (`self.Lever`)))))
  (return (or (and (< _relativerotation_pitch_2 0.0) (> _relativelocation_y_2 0.0)) (and (> _relativerotation_pitch 0.0) (< _relativelocation_y 0.0)))))

(fn `ReduceDiameter`
  (bind _orb (`self.ORB`))
  (set `/Game/Actors/BP_ORB.Diameter` (`KismetMathLibrary.FClamp` (- (`/Game/Actors/BP_ORB.Diameter` _orb) (`KismetMathLibrary.Abs` (`KismetMathLibrary.Conv_IntToDouble` (* (`/Game/Actors/BP_Lever.LeverState` (`self.Lever`)) 2)))) 0.0 300.0) _orb))

(fn `SetStable`
  (set `self.bStabilizing` true)
  (`TimelineComponent.Stop` (`self.TargetE_T`))
  (`TimelineComponent.Stop` (`self.OrbActive`))
  (`TimelineComponent.PlayFromStart` (`self.Stabilzation`)))

(fn `SetUnstable`
  (set `self.bStabilizing` false)
  (`TimelineComponent.Play` (`self.TargetE_T`))
  (`TimelineComponent.PlayFromStart` (`self.OrbActive`))
  (`TimelineComponent.Stop` (`self.Stabilzation`)))

(fn `SetupManifestWidget`
  (bind _returnvalue (`|CreateWidget` "/Game/UI/WBP_Manifests.WBP_Manifests_C"))
  (bind _output_get (set `self.ManifestUI` _returnvalue))
  (`Widget.SetVisibility` _output_get "Collapsed")
  (`UserWidget.AddToViewport` _output_get 0))

(fn `SpeedDriver`
  (bind _returnvalue (`MaterialInstanceDynamic.K2_GetScalarParameterValue` (`/Game/Actors/BP_ORB.OrbGlow` (`self.ORB`)) "SpeedX"))
  (bind _returnvalue_2 (`MaterialInstanceDynamic.K2_GetScalarParameterValue` (`/Game/Actors/BP_ORB.OrbGlow` (`self.ORB`)) "SpeedY"))
  (`/Game/Actors/BP_ORB.SpeedControl` (`self.ORB`) (`KismetMathLibrary.FInterpTo_Constant` _returnvalue 4.0 (`GameplayStatics.GetWorldDeltaSeconds`) 0.5) (`KismetMathLibrary.FInterpTo_Constant` _returnvalue_2 2.0 (`GameplayStatics.GetWorldDeltaSeconds`) 0.5)))

(fn `Stabilize`
  (bind _returnvalue (/ (`KismetMathLibrary.Conv_IntToDouble` (+ (`self.ToStabilization`) 2)) 20.0))
  (if (>= (`self.ToStabilization`) 45)
    (`self.SetStable`)
    (else
      (`/Engine/EditorBlueprintResources/StandardMacros.IncrementInt` (`self.ToStabilization`)
        (:`  `
          (`/Game/Actors/BP_ORB.SpeedControl` (`self.ORB`) _returnvalue (/ _returnvalue 2.0)))))))

(fn `StartEngine`
  (`/Game/Actors/BP_ORB.EnergyDriver` (`self.ORB`))
  (`TimelineComponent.PlayFromStart` (`self.TargetE_T`)))

(fn `Unstabilize`
  (params (StepAmount :type "Float (double-precision)"))
  (set `self.ToStabilization` (`KismetMathLibrary.FTrunc` (`KismetMathLibrary.FClamp` (- (`KismetMathLibrary.Conv_IntToDouble` (`self.ToStabilization`)) (* (`self.Unstabilization`) 0.066667 StepAmount)) 0.0 45.0))))

(fn `UserConstructionScript`)